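; BP_SpikeTrap is a floor spike trap that damages the first-person character on overlap.
; Each overlap applies SpikeDamage and, unless the trap is already active, plays a timeline that moves the spike mesh along Z.
; Its construction script sizes base and spikes from a parent BP_Platfrom_Cell's GridSize and lowers the spikes.
; On BeginPlay it binds to Spike_Trap_Disabler, destroying itself when traps are disabled.
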(event `self.ReceiveBeginPlay`
  (bind _returnvalue (`GameplayStatics.GetActorOfClass` "/Game/blueprints/Spike_Trap_Disabler.Spike_Trap_Disabler_C"))
  (add `/Game/blueprints/Spike_Trap_Disabler.Traps_Disabled` _returnvalue (delegate `disabled`)))

(event `disabled`
  (`self.K2_DestroyActor`))

(event `self.ReceiveActorBeginOverlap`
  (params (OtherActor :type "Actor Object Reference"))
  (bind _opm0041 (`self.OPM0041`))
  (bind (_returnvalue_x _returnvalue_y _returnvalue_z) (`KismetMathLibrary.BreakVector` (`SceneComponent.GetUpVector` _opm0041)))
  (bind _asbp_first_person_character (cast `/Game/FirstPerson/Blueprints/BP_FirstPersonCharacter` OtherActor))
  (bind _output_get (set `self.As BP First Person Character` _asbp_first_person_character))
  (`|ExecutionSequence`
    (:`then_0`
      (if (not (`self.trap active`))
        (bind (_direction _newtrack_0) (`Timeline|spike_up` :!via `PlayFromStart`)
          (:`Update`
            (set `self.trap active` true)
            (`SceneComponent.K2_SetRelativeLocation` _opm0041 (`KismetMathLibrary.MakeVector` _returnvalue_x _returnvalue_y (+ (* _newtrack_0 10.0) _returnvalue_z)) false false))
          (:`Finished`
            (set `self.trap active` false)))))
    (:`then_1`
      (`/Game/FirstPerson/Blueprints/BP_FirstPersonCharacter.Damage_Function` _output_get (`self.Spike_Damage`)))))

(fn `UserConstructionScript`
  (bind _opm0041 (`self.OPM0041`))
  (bind _asbp_platfrom_cell (cast `/Game/blueprints/BP_Platfrom_Cell` (`self.GetParentActor`)))
  (bind _returnvalue (* (`/Game/blueprints/BP_Platfrom_Cell.GridSize` _asbp_platfrom_cell) 0.7))
  (`SceneComponent.SetRelativeScale3D` (`self.Cube`) (`KismetMathLibrary.MakeVector` _returnvalue _returnvalue 0.1))
  (`SceneComponent.SetRelativeScale3D` _opm0041 (`KismetMathLibrary.MakeVector` _returnvalue _returnvalue 5.0))
  (`SceneComponent.K2_SetRelativeLocation` _opm0041 (0.0 0.0 -100.0) false false))