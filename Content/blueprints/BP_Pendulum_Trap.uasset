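; Pendulum sword trap, built to be a child actor of BP_Platfrom_Cell, that damages the first-person character.
; The construction script fits the blade and trigger box to the parent cell's wall height, grid size and trap rotation.
; Player overlap plays the Swing timeline to roll the blade, guarded by TrapActive, and SwordBox overlap applies SwordDamage.
; It destroys itself when Pnedulum_Trap_Disabler broadcasts TrapsDisabled.
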(event `self.ReceiveBeginPlay`
  (add `PrimitiveComponent.OnComponentBeginOverlap` (`self.Trigger_box`) (delegate `OnComponentBeginOverlap_Event`))
  (add `PrimitiveComponent.OnComponentBeginOverlap` (`self.Sword_box`) (delegate `Sword_hit`))
  (bind _returnvalue (`GameplayStatics.GetActorOfClass` "/Game/blueprints/Pnedulum_Trap_Disabler.Pnedulum_Trap_Disabler_C"))
  (add `/Game/blueprints/Pnedulum_Trap_Disabler.Traps_Disabled` _returnvalue (delegate `Disabled`)))

(event `Disabled`
  (`self.K2_DestroyActor`))

(event `OnComponentBeginOverlap_Event`
  (params (OverlappedComponent :type "PrimitiveComponent Object Reference") (OtherActor :type "Actor Object Reference") (OtherComp :type "PrimitiveComponent Object Reference") (OtherBodyIndex :type Integer) (bFromSweep :type Boolean) (SweepResult :type "HitResult Structure (by ref)"))
  (bind (_trap_rotation_roll _trap_rotation_pitch _trap_rotation_yaw) (`KismetMathLibrary.BreakRotator` (`/Game/blueprints/BP_Platfrom_Cell.Trap_Rotation` (`self.Cell_Ref`))))
  (cast `/Game/FirstPerson/Blueprints/BP_FirstPersonCharacter` OtherActor)
  (if (not (`self.Trap_active`))
    (bind (_direction _newtrack_0) (`Timeline|Swing` :!via `PlayFromStart`)
      (:`Update`
        (set `self.Trap_active` true)
        (`SceneComponent.K2_SetRelativeRotation` (`self.sworb`) (`KismetMathLibrary.MakeRotator` (+ (* _newtrack_0 45.0) 0.0) 180.0 _trap_rotation_yaw) false false))
      (:`Finished`
        (set `self.Trap_active` false)))))

(event `Sword_hit`
  (params (OverlappedComponent :type "PrimitiveComponent Object Reference") (OtherActor :type "Actor Object Reference") (OtherComp :type "PrimitiveComponent Object Reference") (OtherBodyIndex :type Integer) (bFromSweep :type Boolean) (SweepResult :type "HitResult Structure (by ref)"))
  (bind _asbp_first_person_character (cast `/Game/FirstPerson/Blueprints/BP_FirstPersonCharacter` OtherActor))
  (`/Game/FirstPerson/Blueprints/BP_FirstPersonCharacter.Damage_Function` _asbp_first_person_character (`self.Sword_damage`)))

(fn `Get_Interact_State`
  (returns (InteractState :type Boolean))
  (return false))

(fn `UserConstructionScript`
  (bind _sworb (`self.sworb`))
  (bind _gridsize (`/Game/blueprints/BP_Platfrom_Cell.GridSize` (`self.Cell_Ref`)))
  (bind (_trap_rotation_roll _trap_rotation_pitch _trap_rotation_yaw) (`KismetMathLibrary.BreakRotator` (`/Game/blueprints/BP_Platfrom_Cell.Trap_Rotation` (`self.Cell_Ref`))))
  (bind _asbp_platfrom_cell (cast `/Game/blueprints/BP_Platfrom_Cell` (`self.GetParentActor`)))
  (bind _output_get (set `self.Cell_Ref` _asbp_platfrom_cell))
  (`|ExecutionSequence`
    (:`then_0`
      (bind _wall_height (`/Game/blueprints/BP_Platfrom_Cell.wall_height` _output_get))
      (`SceneComponent.K2_SetRelativeLocation` _sworb (`KismetMathLibrary.MakeVector` 0.0 0.0 (* _wall_height 100.0)) false false)
      (`SceneComponent.SetRelativeScale3D` _sworb (`KismetMathLibrary.Conv_DoubleToVector` (* _wall_height 0.05)))
      (`SceneComponent.K2_SetRelativeRotation` _sworb (`KismetMathLibrary.MakeRotator` 45.0 _trap_rotation_pitch _trap_rotation_yaw) false false))
    (:`then_1`
      (`SceneComponent.SetRelativeScale3D` (`self.Trigger_box`) (`KismetMathLibrary.MakeVector` _gridsize _gridsize 0.1)))))