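; BP_Keys is a colored key pickup that spins continuously on a looping timeline until collected.
; The construction script sets its material and color name from the Color variable.
; Interacting adds that name to the first-person character's Keys, prints a message and destroys the key.
; At BeginPlay it binds to the player's time-slow event, which lowers or restores the key's custom time dilation.
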(event `self.ReceiveBeginPlay`
  (bind _key (`self.key`))
  (bind (_relativelocation_x _relativelocation_y) (`KismetMathLibrary.BreakVector` (`SceneComponent.RelativeLocation` _key)))
  (bind _returnvalue (`GameplayStatics.GetActorOfClass` "/Game/GameDev2_Labwork_Assets/blueprints/BP_FirstPersonCharacter.BP_FirstPersonCharacter_C"))
  (bind _output_get (set `self.PlayerRef` _returnvalue))
  (add `/Game/GameDev2_Labwork_Assets/blueprints/BP_FirstPersonCharacter.Time_Slow` _output_get (delegate `Time Slow`))
  (bind (_direction _rotate) (`Timeline|Animation` :!label _label)
    (:`Update`
      (`SceneComponent.K2_SetRelativeLocation` _key (`KismetMathLibrary.MakeVector` _relativelocation_x _relativelocation_y 100.0) false false)
      (bind _returnvalue_2 (* _rotate 90.0))
      (`SceneComponent.K2_SetRelativeRotation` _key (`KismetMathLibrary.MakeRotator` 0.0 _returnvalue_2 _returnvalue_2) false false))
    (:`Finished`
      (goto _label :!via `PlayFromStart`))))

(event `/Game/GameDev2_Labwork_Assets/blueprints/Interface_Test.Interact`
  (params (NewParam :type "PrimitiveComponent Object Reference"))
  (bind _keycolorname (`self.KeyColorName`))
  (`KismetArrayLibrary.Array_Add` (`/Game/GameDev2_Labwork_Assets/blueprints/BP_FirstPersonCharacter.Keys` (`self.PlayerRef`)) _keycolorname)
  (`KismetSystemLibrary.PrintString` (`KismetStringLibrary.Concat_StrStr` _keycolorname " key acquired"))
  (`self.K2_DestroyActor`))

(event `Time Slow`
  (params (NewParam :type Boolean))
  (if NewParam
    (set `self.CustomTimeDilation` 0.2)
    (else
      (set `self.CustomTimeDilation` 1.0))))

(fn `Get_Interact_State`
  (returns (InteractState :type Boolean))
  (return false))

(fn `UserConstructionScript`
  (bind _color (`self.Color`))
  (`PrimitiveComponent.SetMaterial` (`self.key`) 0 (select `/Game/GameDev2_Labwork_Assets/blueprints/color` _color :`NewEnumerator0` "/Game/GameDev2_Labwork_Assets/materials/red.red" :`NewEnumerator1` "/Game/GameDev2_Labwork_Assets/materials/green.green" :`NewEnumerator2` "/Game/GameDev2_Labwork_Assets/materials/blue.blue" :!type "MaterialInterface Object Reference"))
  (set `self.KeyColorName` (select `/Game/GameDev2_Labwork_Assets/blueprints/color` _color :`NewEnumerator0` "red" :`NewEnumerator1` "green" :`NewEnumerator2` "blue")))