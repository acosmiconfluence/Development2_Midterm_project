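; A color-keyed door that the player opens and closes through interaction once they hold the matching key.
; The construction script sets the material and required key name from the Color choice.
; Interact searches the player character's Keys for that name, then a FlipFlop plays or reverses a timeline that slides the mesh vertically.
; It binds to the character's time-slow event to lower its own CustomTimeDilation.
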(event `self.ReceiveBeginPlay`
  (bind _returnvalue (`GameplayStatics.GetActorOfClass` "/Game/GameDev2_Labwork_Assets/blueprints/BP_FirstPersonCharacter.BP_FirstPersonCharacter_C"))
  (bind _output_get (set `self.CharacterRef` _returnvalue))
  (add `/Game/GameDev2_Labwork_Assets/blueprints/BP_FirstPersonCharacter.Time_Slow` _output_get (delegate `Time_Slow`)))

(event `Time_Slow`
  (params (NewParam :type Boolean))
  (if NewParam
    (set `self.CustomTimeDilation` 0.2)
    (else
      (set `self.CustomTimeDilation` 1.0))))

(event `/Game/GameDev2_Labwork_Assets/blueprints/Interface_Test.Interact`
  (params (NewParam :type "PrimitiveComponent Object Reference"))
  (for _array_element (`/Game/GameDev2_Labwork_Assets/blueprints/BP_FirstPersonCharacter.Keys` (`self.CharacterRef`))
    (if (`KismetStringLibrary.EqualEqual_StrStr` _array_element (`self.DoorColor`))
      (set `self.door_unlocked` true)))
  (if (`self.door_unlocked`)
    (`KismetSystemLibrary.PrintString` "Door Unlocked")
    (`/Engine/EditorBlueprintResources/StandardMacros.FlipFlop`
      (:`A`
        (bind (_direction _rotation) (`Timeline|Door_Anim` :!via `PlayFromStart` :!label _label)
          (:`Update`
            (`SceneComponent.K2_SetRelativeLocation` (`self.StaticMesh`) (`KismetMathLibrary.VLerp` (0.0 0.0 0.0) (0.0 0.0 450.0) _rotation) false false))))
      (:`B`
        (goto _label :!via `Reverse`)))
    (else
      (`KismetSystemLibrary.PrintString` "You Dont Have The Correct Key"))))

(fn `Get_Interact_State`
  (returns (InteractState :type Boolean))
  (return false))

(fn `UserConstructionScript`
  (bind _color (`self.Color`))
  (set `self.MaterialRef` (select `/Game/GameDev2_Labwork_Assets/blueprints/color` _color :`NewEnumerator0` "/Game/GameDev2_Labwork_Assets/materials/red.red" :`NewEnumerator1` "/Game/GameDev2_Labwork_Assets/materials/green.green" :`NewEnumerator2` "/Game/GameDev2_Labwork_Assets/materials/blue.blue" :!type "MaterialInterface Object Reference"))
  (set `self.DoorColor` (select `/Game/GameDev2_Labwork_Assets/blueprints/color` _color :`NewEnumerator0` "red" :`NewEnumerator1` "green" :`NewEnumerator2` "blue"))
  (`PrimitiveComponent.SetMaterial` (`self.StaticMesh`) 0 (`self.MaterialRef`)))