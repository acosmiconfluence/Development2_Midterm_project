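; Spike trap that sizes itself to its parent BP_Platfrom_Cell and damages the player through a hitbox.
; Player overlap with the trigger starts a short delay, then a Timeline moves the spikes.
; The player's time-slow event lowers the trap's CustomTimeDilation, revealing Spike2 mid-animation as a one-time interactable that calls the player's Gaze.
; A BP_Trap_Disabler with index 0 can temporarily disable the trap and swap its material.
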(event `self.ReceiveBeginPlay`
  ;[0.2399 1 0] Begin Play Setup
  (bind _asbp_first_person_character (cast `/Game/GameDev2_Labwork_Assets/blueprints/BP_FirstPersonCharacter` (`GameplayStatics.GetPlayerCharacter` 0)))
  (bind _output_get (set `self.As BP First Person Character` _asbp_first_person_character))
  (add `/Game/GameDev2_Labwork_Assets/blueprints/BP_FirstPersonCharacter.Time_Slow` _output_get (delegate `Time_Slow`))
  (bind _outactors (`GameplayStatics.GetAllActorsOfClass` "/Game/GameDev2_Labwork_Assets/blueprints/BP_Trap_Disabler.BP_Trap_Disabler_C"))
  (for _array_element _outactors
    (if (== (`/Game/GameDev2_Labwork_Assets/blueprints/BP_Trap_Disabler.Target_trap_index` _array_element) 0)
      (set `self.Disabler_Ref` _array_element)))
  (add `/Game/GameDev2_Labwork_Assets/blueprints/BP_Trap_Disabler.Traps_Disabled` (`self.Disabler_Ref`) (delegate `disabled`)))

(event `Time_Slow`
  (params (NewParam :type Boolean))
  ;[1 0.008642 0] Time Slow
  (if NewParam
    (set `self.CustomTimeDilation` 0.2)
    (set `self.Time_Is_Slowed` true)
    (else
      (set `self.CustomTimeDilation` 1.0)
      (set `self.Time_Is_Slowed` false))))

(event `disabled`
  (params (Trap_Target_Index :type Integer))
  ;[1 0.0179 0] Disabled
  (if (== Trap_Target_Index 0)
    (set `self.Is_Enabled` false)
    (`PrimitiveComponent.SetMaterial` (`self.Cube`) 0 "/Interchange/gltf/M_Default.M_Default")
    (`KismetSystemLibrary.Delay` 8.0)
    (set `self.Is_Enabled` true)
    (`PrimitiveComponent.SetMaterial` (`self.Cube`) 0 "/Game/GameDev2_Labwork_Assets/materials/red.red")))

(event `self.trap_trigger.OnComponentBeginOverlap`
  (params (OverlappedComponent :type "PrimitiveComponent Object Reference") (OtherActor :type "Actor Object Reference") (OtherComp :type "PrimitiveComponent Object Reference") (OtherBodyIndex :type Integer) (bFromSweep :type Boolean) (SweepResult :type "HitResult Structure (by ref)"))
  (bind _opm0041 (`self.OPM0041`))
  (bind _spike2 (`self.Spike2`))
  (bind _time_is_slowed (`self.Time_Is_Slowed`))
  (bind _spike2_2 (`self.Spike2`))
  (bind (_returnvalue_x _returnvalue_y _returnvalue_z) (`KismetMathLibrary.BreakVector` (* (`SceneComponent.GetUpVector` _opm0041) (0.0 0.0 0.0))))
  ;[1 0 0] Trap Trigger
  (if (== OtherActor (`self.As BP First Person Character`))
    (if (`self.Is_Enabled`)
      (if (not (`self.trap_anim_active`))
        (`KismetSystemLibrary.Delay` 0.3)
        ;[1 1 1] Trap Animation
        (bind (_direction _newtrack_0) (`Timeline|Timeline` :!via `PlayFromStart`)
          (:`Update`
            (set `self.trap_anim_active` true)
            (`SceneComponent.K2_SetRelativeLocation` _opm0041 (`KismetMathLibrary.MakeVector` _returnvalue_x _returnvalue_y (+ (* _newtrack_0 10.0) _returnvalue_z)) false false)
            (if (`KismetSystemLibrary.IsValid` _spike2)
              (`SceneComponent.SetVisibility` _spike2 _time_is_slowed false)
              (set `self.Spike_Interactable` _time_is_slowed)))
          (:`Finished`
            (set `self.trap_anim_active` false)
            (set `self.Spike_Interactable` false)
            (if (`KismetSystemLibrary.IsValid` _spike2_2)
              (`SceneComponent.SetVisibility` _spike2_2 false false))))))))

(event `self.spike_hitbox.OnComponentBeginOverlap`
  (params (OverlappedComponent :type "PrimitiveComponent Object Reference") (OtherActor :type "Actor Object Reference") (OtherComp :type "PrimitiveComponent Object Reference") (OtherBodyIndex :type Integer) (bFromSweep :type Boolean) (SweepResult :type "HitResult Structure (by ref)"))
  (bind _as_bp_first_person_character (`self.As BP First Person Character`))
  ;[1 0.03273 0] Spike Hitbox
  (if (== OtherActor _as_bp_first_person_character)
    (`/Game/GameDev2_Labwork_Assets/blueprints/BP_FirstPersonCharacter.Damage_Function` _as_bp_first_person_character (`self.Spike_Damage`))))

(event `/Game/GameDev2_Labwork_Assets/blueprints/Interface_Test.Interact`
  (params (NewParam :type "PrimitiveComponent Object Reference"))
  (if (`self.Spike_Interactable`)
    (`KismetSystemLibrary.PrintString` "Hello")
    (`/Engine/EditorBlueprintResources/StandardMacros.DoOnce` false
      (:`Completed`
        (`ActorComponent.K2_DestroyComponent` (`self.Spike2`))
        (`/Game/GameDev2_Labwork_Assets/blueprints/BP_FirstPersonCharacter.Gaze` (`self.As BP First Person Character`))))
    (else
      (`KismetSystemLibrary.PrintString` "f"))))

(fn `Get_Interact_State`
  (returns (InteractState :type Boolean))
  (return false))

(fn `UserConstructionScript`
  (bind _opm0041 (`self.OPM0041`))
  (bind _asbp_platfrom_cell (cast `/Game/GameDev2_Labwork_Assets/blueprints/BP_Platfrom_Cell` (`self.GetParentActor`)))
  (bind _gridsize (`/Game/GameDev2_Labwork_Assets/blueprints/BP_Platfrom_Cell.GridSize` _asbp_platfrom_cell))
  (bind _returnvalue (* _gridsize 1.0))
  (`SceneComponent.SetRelativeScale3D` (`self.Cube`) (`KismetMathLibrary.MakeVector` _returnvalue _returnvalue 0.1))
  (bind _returnvalue_2 (* _gridsize 1.5))
  (`SceneComponent.SetRelativeScale3D` (`self.trap_trigger`) (`KismetMathLibrary.MakeVector` _returnvalue_2 _returnvalue_2 1.0))
  (`SceneComponent.SetRelativeScale3D` _opm0041 (`KismetMathLibrary.MakeVector` _returnvalue _returnvalue 5.0))
  (`SceneComponent.K2_SetRelativeLocation` _opm0041 (0.0 0.0 -100.0) false false))